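; BP_Paint is a movable brush actor that paints onto BP_Canvas render targets, moved along three axes by input.
; While its cube overlaps something, Tick line-traces along the cube's right axis against WorldStatic objects and finds the hit UV.
; That UV sets the Position of a dynamic M_Paint material, which is drawn into the canvas's render target.
; The construction script creates that material with the brush size and optional paint texture.
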(event `InputAxis|MovePaintForward`
  (params (AxisValue :type "Float (single-precision)"))
  ;[1 1 1] 移动cube
  (`SceneComponent.K2_AddRelativeLocation` (`self.DefaultSceneRoot`) (* (`self.PaintForwardSpeed`) AxisValue) false false))

(event `InputAxis|MovePaintRight`
  (params (AxisValue :type "Float (single-precision)"))
  ;[1 1 1] 移动cube
  (`SceneComponent.K2_AddRelativeLocation` (`self.DefaultSceneRoot`) (* (`self.PaintRightSpeed`) AxisValue) false false))

(event `InputAxis|MovePaintIn`
  (params (AxisValue :type "Float (single-precision)"))
  ;[1 1 1] 移动cube
  (`SceneComponent.K2_AddRelativeLocation` (`self.DefaultSceneRoot`) (* (`self.PaintInSpeed`) AxisValue) false false))

(event `self.ReceiveTick`
  (params (DeltaSeconds :type "Float (single-precision)"))
  (bind _cube (`self.Cube`))
  (bind _returnvalue (`SceneComponent.K2_GetComponentLocation` _cube))
  (bind _returnvalue_2 (`KismetMathLibrary.GetRightVector` (`SceneComponent.K2_GetComponentRotation` _cube)))
  (if (`self.IsOverlap`)
    (bind (_outhit _returnvalue_3) (`KismetSystemLibrary.LineTraceSingleForObjects` :`Start` (+ _returnvalue (* _returnvalue_2 100.0)) :`End` (+ (* _returnvalue_2 -1000.0) _returnvalue) :`ObjectTypes` (`|MakeArray` "ObjectTypeQuery1" :!type "EObjectTypeQuery Enum") :`bTraceComplex` true :`DrawDebugType` "ForOneFrame"))
    (if _returnvalue_3
      (bind _asbp_canvas (cast `/Game/Painting/BP_Canvas` (`.HitActor` (`GameplayStatics.BreakHitResult` _outhit))))
      (bind _uv (`GameplayStatics.FindCollisionUV` _outhit))
      (`MaterialInstanceDynamic.SetVectorParameterValue` (`self.m_Paint`) "Position" (make `LinearColor` (`KismetMathLibrary.BreakVector2D` _uv) (`.Y` (`KismetMathLibrary.BreakVector2D` _uv)) 0.0 1.0))
      (`KismetRenderingLibrary.DrawMaterialToRenderTarget` (`/Game/Painting/BP_Canvas.RenderTex` _asbp_canvas) (`self.m_Paint`)))))

(event `self.Cube.OnComponentBeginOverlap`
  (params (OverlappedComponent :type "PrimitiveComponent Object Reference") (OtherActor :type "Actor Object Reference") (OtherComp :type "PrimitiveComponent Object Reference") (OtherBodyIndex :type Integer) (bFromSweep :type Boolean) (SweepResult :type "HitResult Structure (by ref)"))
  ;[1 1 1] 检测在碰撞范围内
  (set `self.IsOverlap` true))

(event `self.Cube.OnComponentEndOverlap`
  (params (OverlappedComponent :type "PrimitiveComponent Object Reference") (OtherActor :type "Actor Object Reference") (OtherComp :type "PrimitiveComponent Object Reference") (OtherBodyIndex :type Integer))
  ;[1 1 1] 检测在碰撞范围内
  (set `self.IsOverlap` false))

(fn `UserConstructionScript`
  (bind _paintex (`self.PainTex`))
  (bind _returnvalue (`KismetMaterialLibrary.CreateDynamicMaterialInstance` "/Game/Painting/M_Paint.M_Paint"))
  (bind _output_get (set `self.m_Paint` _returnvalue))
  (`MaterialInstanceDynamic.SetScalarParameterValue` _output_get "Size" (`self.PaintSize`))
  (`/Engine/EditorBlueprintResources/StandardMacros.IsValid` _paintex
    (:`Is Valid`
      (`MaterialInstanceDynamic.SetTextureParameterValue` _output_get "PaintTex" _paintex))))